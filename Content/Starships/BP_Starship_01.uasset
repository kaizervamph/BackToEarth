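; BP_Starship_01 is a starship Blueprint with left and right weapons mounted as child actors.
; PrepareWeapons casts each to BP_StarshipWeaponBase and starts its cooldown, followed by an IsPlayer check that does nothing.
; The construction script only calls its parent; a disconnected loop that would apply M_Test to child static meshes never runs.
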(event EventBeginPlay)

(event Collision|EventActorBeginOverlap
  (params (OtherActor :type Actor%20Object%20Reference)))

(event EventTick
  (params (DeltaSeconds :type Float%20%28single-precision%29)))

(event EventPrepareWeapons
  (for _array_element (Utilities|Array|MakeArray (Variables|/Script/Engine.ChildActorComponent|GetChildActor (Variables|Default|GetWeapon_Right)) (Variables|/Script/Engine.ChildActorComponent|GetChildActor (Variables|Default|GetWeapon_Left)))
    (bind _asbp_starship_weapon_base (Utilities|Casting|CastToBP_StarshipWeaponBase _array_element))
    (Default|StartCooldown _asbp_starship_weapon_base)
    (if (Variables|Default|GetIsPlayer)
      _)))

(fn ConstructionScript
  (|CallParentFunction))