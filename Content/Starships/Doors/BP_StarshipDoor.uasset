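; BP_StarshipDoor is an interactable starship door that units can open and close.
; Its Box trigger registers the door as the interact object on overlapping BP_UnitBase actors and clears it when they leave.
; Interacting flip-flops a timeline that moves the Door mesh vertically and updates DoorOpen from the playback direction.
; The construction script sizes and positions the door, surrounding cubes and trigger from size variables.
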(event OnComponentBeginOverlap(Box)
  (params (OverlappedComponent :type Primitive%20Component%20Object%20Reference) (OtherActor :type Actor%20Object%20Reference) (OtherComp :type Primitive%20Component%20Object%20Reference) (OtherBodyIndex :type Integer) (bFromSweep :type Boolean) (SweepResult :type Hit%20Result%20Structure%20%28by%20ref%29))
  (bind _asbp_unit_base (Utilities|Casting|CastToBP_UnitBase OtherActor))
  (Default|SetInteractObject _asbp_unit_base self))

(event OnComponentEndOverlap(Box)
  (params (OverlappedComponent :type Primitive%20Component%20Object%20Reference) (OtherActor :type Actor%20Object%20Reference) (OtherComp :type Primitive%20Component%20Object%20Reference) (OtherBodyIndex :type Integer))
  (bind _asbp_unit_base (Utilities|Casting|CastToBP_UnitBase OtherActor))
  (Default|SetInteractObject _asbp_unit_base))

(event Custom|ToggleState
  (Utilities|FlowControl|FlipFlop
    (:A
      (bind (_direction _location) (Timeline|ToggleStateDoor Play)
        (:Update
          (Transformation|SetRelativeLocation (Variables|Default|GetDoor) (Math|Vector|MakeVector 0.0 0.0 (+ _location 1.5e+02)) false false)
          (switch Utilities|FlowControl|Switch|SwitchonETimelineDirection _direction
            (:Forward
              (Variables|Default|SetDoorOpen? true))
            (:Backward
              (Variables|Default|SetDoorOpen? false))))))
    (:B
      (Timeline|ToggleStateDoor Reverse))))

(event EventBeginPlay)

(event Collision|EventActorBeginOverlap
  (params (OtherActor :type Actor%20Object%20Reference)))

(event EventTick
  (params (DeltaSeconds :type Float%20%28single-precision%29)))

(event EventInteractwithObject
  (params (Unit :type BP%20Unit%20Base%20Object%20Reference))
  (CallFunction|ToggleState))

(fn ConstructionScript
  (bind _sizex (Variables|Default|GetSizeX))
  (bind _sizez (Variables|Default|GetSizeZ))
  (bind _box (Variables|Default|GetBox))
  (bind _returnvalue (* _sizex 1e+02))
  (bind _boxextent (Variables|/Script/Engine.BoxComponent|GetBoxExtent _box))
  (bind _returnvalue_2 (/ _returnvalue 2.0))
  (bind (_x _y) (Math|Vector|BreakVector _boxextent))
  (bind _returnvalue_3 (+ _returnvalue_2 5e+01))
  (Transformation|SetRelativeScale3D (Variables|Default|GetCube) (Math|Vector|MakeVector (Variables|Default|GetSizeX) (Variables|Default|GetSizeY) 0.1))
  (Components|Box|SetBoxExtent _box (Math|Vector|MakeVector _x _y _sizez) true)
  (Transformation|SetRelativeLocation _box (Math|Vector|MakeVector 0.0 0.0 _sizez) false false)
  (Transformation|SetRelativeLocation (Variables|Default|GetCube1) (Math|Vector|MakeVector _returnvalue_3 0.0 1.5e+02) false false)
  (bind _result (Math|Float|NegateFloat _returnvalue_3)
    (:%20%20
      (Transformation|SetRelativeLocation (Variables|Default|GetCube2) (Math|Vector|MakeVector _result 0.0 1.5e+02) false false)
      (Transformation|SetRelativeScale3D (Variables|Default|GetCube3) (Math|Vector|MakeVector (+ (Variables|Default|GetSizeX) 2.0) (Variables|Default|GetSizeY) 1.0))
      (Transformation|SetRelativeScale3D (Variables|Default|GetDoor) (Math|Vector|MakeVector (Variables|Default|GetSizeX) 0.5 3.0)))))