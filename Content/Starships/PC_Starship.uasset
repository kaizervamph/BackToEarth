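; Player controller for the starship that highlights floor meshes under the mouse cursor.
; Each tick HoverMouse traces the Visibility channel with complex collision and, when the hit component changes, switches the highlight from HoveredMesh to any static mesh component tagged "Floor".
; HoverFXinMesh drives the highlight by toggling Render Custom Depth.
; Each newly hovered floor mesh also prints its socket names as debug output.
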(event Custom|HoverMouse
  (bind _hitresult (Game|Player|GetHitResultUnderCursorbyChannel "TraceTypeQuery1" true))
  (bind _hitcomponent (Collision|BreakHitResult _hitresult))
  (bind _hoveredmesh (Variables|Default|GetHoveredMesh)
    (:then
      (if (not (== _hoveredmesh _hitcomponent))
        (CallFunction|HoverFXinMesh _hoveredmesh false)
        (bind _ascomponente_de_malla_estática (Utilities|Casting|CastToStaticMeshComponent _hitcomponent :!label _label))
        (if (Components|ComponentHasTag _ascomponente_de_malla_estática "Floor")
          (bind _output_get (Variables|Default|SetHoveredMesh _ascomponente_de_malla_estática))
          (CallFunction|HoverFXinMesh _output_get true)
          (for _array_element (Transformation|GetAllSocketNames _output_get)
            (Development|PrintString (Utilities|String|ToString(Name) _array_element))))))
    (:else
      (goto _label))))

(event EventBeginPlay)

(event EventTick
  (params (DeltaSeconds :type Float%20%28single-precision%29))
  (CallFunction|HoverMouse))

(fn ConstructionScript)

(fn HoverFXinMesh
  (params (HoveredMesh :type Static%20Mesh%20Component%20Object%20Reference) (Value :type Boolean))
  (Rendering|SetRenderCustomDepth HoveredMesh Value)
  (return true))