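; Base starship actor that holds shield and fuel state and handles travel between space locations.
; On BeginPlay it seeds current and maximum shield and fuel from StarshipInfo.
; TravelToSpace deducts fuel, closes the interstellar map widget, restores game-only input and has each BP_SolarSystem load the destination.
; Modules and doors are child actor components, gathered by helper functions into maps of actor to relative location.
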(event Custom|SetDefaultValues
  (bind _starshipinfo (Variables|Default|GetStarshipInfo))
  (bind (_name _shield _fuel) (Utilities|Struct|BreakStarshipStruct _starshipinfo))
  (Variables|Default|SetShield _shield)
  (Variables|Default|SetShieldMax _shield)
  (Variables|Default|SetFuel _fuel)
  (Variables|Default|SetFuelMax _fuel))

(event Custom|TravelToSpace
  (params (SpaceLocation :type Space%20Location%20Struct%20Structure) (FuelCost :type Float%20%28single-precision%29))
  (Variables|Default|SetFuel (- (Variables|Default|GetFuel) FuelCost))
  (bind _foundwidgets (Widget|GetAllWidgetsOfClass "/Game/Gameplay/UI/WBP_InterestelarMap.WBP_InterestelarMap_C" false))
  (for _array_element _foundwidgets
    (Widget|RemovefromParent _array_element)
    (Input|SetInputModeGameOnly (Game|GetPlayerController 0))
    (Utilities|Platform|CollectGarbage))
  (bind _outactors (Actor|GetAllActorsOfClass "/Game/Levels/BP_SolarSystem.BP_SolarSystem_C"))
  (for _array_element_2 _outactors
    (Default|LoadSpaceLocation _array_element_2 SpaceLocation)))

(event EventBeginPlay
  (CallFunction|SetDefaultValues))

(fn ConstructionScript)

(fn GetAllModules
  (for _array_element (Components|GetChildrenComponents (Variables|Default|GetDefaultSceneRoot) true)
    (bind _ascomponente_de_actor_hijo (Utilities|Casting|CastToChildActorComponent _array_element))
    (bind _asbp_module_base (Utilities|Casting|CastToBP_ModuleBase (Variables|/Script/Engine.ChildActorComponent|GetChildActor _ascomponente_de_actor_hijo)))
    (Utilities|Map|Add (LocalVariables|GetTemp) _asbp_module_base (.Location (Math|Transform|BreakTransform (Transformation|GetRelativeTransform _ascomponente_de_actor_hijo)))))
  (return (LocalVariables|GetTemp)))

(fn GetAllDoors
  (for _array_element (Components|GetChildrenComponents (Variables|Default|GetDefaultSceneRoot) true)
    (bind _ascomponente_de_actor_hijo (Utilities|Casting|CastToChildActorComponent _array_element))
    (bind _asbp_starship_door (Utilities|Casting|CastToBP_StarshipDoor (Variables|/Script/Engine.ChildActorComponent|GetChildActor _ascomponente_de_actor_hijo)))
    (Utilities|Map|Add (LocalVariables|GetTemp) _asbp_starship_door (.Location (Math|Transform|BreakTransform (Transformation|GetRelativeTransform _ascomponente_de_actor_hijo)))))
  (return (LocalVariables|GetTemp)))