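; Base starship weapon projectile that damages a single assigned module target on contact.
; SetTargetInfo stores the ModuleTarget, and the Sphere1 overlap handler ignores every other actor.
; A DoOnce gate limits the hit to one trigger, which applies fixed damage, spawns a scaled-up explosion emitter, prints a debug message and destroys the projectile.
; The graph contains no movement logic, and BeginPlay and the construction script are empty.
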(event OnComponentBeginOverlap(Sphere1)
  (params (OverlappedComponent :type Primitive%20Component%20Object%20Reference) (OtherActor :type Actor%20Object%20Reference) (OtherComp :type Primitive%20Component%20Object%20Reference) (OtherBodyIndex :type Integer) (bFromSweep :type Boolean) (SweepResult :type Hit%20Result%20Structure%20%28by%20ref%29))
  (bind _returnvalue (Math|Float|MakeLiteralFloat 5.0))
  (if (== OtherActor (Variables|Default|GetModuleTarget))
    (Utilities|FlowControl|DoOnce false
      (:Completed
        (bind _moduletarget (Variables|Default|GetModuleTarget)
          (:then
            (Game|Damage|ApplyDamage _moduletarget 25.0 0 self)
            (Effects|SpawnEmitteratLocation "/Game/SciFiWeapDark/FX/Particles/P_Grenade_Explosion_Dark.P_Grenade_Explosion_Dark" (Transformation|GetActorLocation) "0, 0, 0" (Math|Vector|MakeVector _returnvalue _returnvalue _returnvalue))
            (Development|PrintString "Projectile HIT" true true "(R=1.000000,G=0.739271,B=0.000000,A=1.000000)" 2222.0)
            (Actor|DestroyActor))
          (:else))))))

(event Custom|SetTargetInfo
  (params (ModuleTarget :type BP%20Module%20Base%20Object%20Reference))
  (Variables|Default|SetModuleTarget ModuleTarget))

(event EventBeginPlay)

(fn ConstructionScript)