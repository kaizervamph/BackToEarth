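; Base actor for starship modules, holding HP and oxygen initialised from its ModuleInfo at BeginPlay.
; The construction script rebuilds a centred SizeX by SizeY grid of tagged floor meshes under SceneFloor and resizes the Box to match.
; Any damage subtracts directly from HP with no clamping or death handling, and getters return current and maximum HP and oxygen.
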(event Custom|SetDefaultValues
  (bind _moduleinfo (Variables|Default|GetModuleInfo))
  (bind (_name _type _hp _oxygen) (Utilities|Struct|BreakModuleStruct _moduleinfo))
  (Variables|Default|SetHP _hp)
  (Variables|Default|SetOxygen _oxygen))

(event EventBeginPlay
  (CallFunction|SetDefaultValues))

(event Game|Damage|EventAnyDamage
  (params (Damage :type Float%20%28single-precision%29) (DamageType :type Damage%20Type%20Object%20Reference) (InstigatedBy :type Controller%20Object%20Reference) (DamageCauser :type Actor%20Object%20Reference))
  (Variables|Default|SetHP (- (Variables|Default|GetHP) Damage)))

(fn ConstructionScript
  (bind _sizez (Variables|Default|GetSizeZ))
  (bind _box (Variables|Default|GetBox))
  (CallFunction|SpawnFloorMeshes)
  (Components|Box|SetBoxExtent _box (Math|Vector|MakeVector (/ (* (Variables|Default|GetSizeX) (Variables|Default|GetSpacing)) 2.0) (/ (* (Variables|Default|GetSizeY) (Variables|Default|GetSpacing)) 2.0) _sizez) true)
  (Transformation|SetRelativeLocation _box (Math|Vector|MakeVector 0.0 0.0 _sizez) false false))

(fn GetValuesHP
  (return (Variables|Default|GetHP) (.HP (Utilities|Struct|BreakModuleStruct (Variables|Default|GetModuleInfo)))))

(fn GetValuesOX
  (return (Variables|Default|GetOxygen) (.Oxygen (Utilities|Struct|BreakModuleStruct (Variables|Default|GetModuleInfo)))))

(fn SpawnFloorMeshes
  (bind _returnvalue (Transformation|GetActorLocation))
  (bind _spacing (Variables|Default|GetSpacing))
  (bind (_x _y _z) (Math|Vector|BreakVector _returnvalue))
  (CallFunction|ClearFloorMeshes)
  (for _index (range 0 (- (Variables|Default|GetSizeX) 1))
    (LocalVariables|SetXvalue _index)
    (for _index_2 (range 0 (- (Variables|Default|GetSizeY) 1))
      (LocalVariables|SetYvalue _index_2)
      (bind _returnvalue_2 (AddComponent|AddStaticMeshComponent true (Math|Transform|MakeTransform (Math|Vector|MakeVector (+ _x (* (LocalVariables|GetXvalue) (Variables|Default|GetSpacing))) (+ _y (* (LocalVariables|GetYvalue) (Variables|Default|GetSpacing))) _z))))
      (Components|StaticMesh|SetStaticMesh _returnvalue_2 (Variables|Default|GetFloorMesh))
      (Variables|/Script/Engine.ActorComponent|SetComponentTags _returnvalue_2 (Utilities|Array|MakeArray "Floor"))
      (Transformation|AttachComponentToComponent _returnvalue_2 (Variables|Default|GetScene_Floor) "None" "KeepWorld" "KeepRelative" "KeepRelative" true)))
  (Transformation|SetRelativeLocation (Variables|Default|GetScene_Floor) (Math|Vector|MakeVector (* (/ (* (Variables|Default|GetSizeX) _spacing) 2.0) -1.0) (* (/ (* (Variables|Default|GetSizeY) _spacing) 2.0) -1.0) 0.0) false false)
  (return true))

(fn ClearFloorMeshes
  (for _array_element (Components|GetChildrenComponents (Variables|Default|GetScene_Floor) false)
    (Components|DestroyComponent _array_element))
  (Transformation|SetRelativeLocation (Variables|Default|GetScene_Floor) "0, 0, 0" false false)
  (return true))