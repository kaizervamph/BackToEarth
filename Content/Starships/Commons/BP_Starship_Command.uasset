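; Starship command actor that toggles the interstellar map UI when a unit interacts with it.
; Sphere overlap begin and end feed UpdateOverlap, and interacting also clears that overlap state for the unit.
; If no map widget exists, it creates one and shows the cursor with Game and UI input.
; Otherwise it removes all map widgets, forces garbage collection and restores game-only input.
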(event OnComponentBeginOverlap(Sphere)
  (params (OverlappedComponent :type Primitive%20Component%20Object%20Reference) (OtherActor :type Actor%20Object%20Reference) (OtherComp :type Primitive%20Component%20Object%20Reference) (OtherBodyIndex :type Integer) (bFromSweep :type Boolean) (SweepResult :type Hit%20Result%20Structure%20%28by%20ref%29))
  (CallFunction|UpdateOverlap OtherActor true))

(event OnComponentEndOverlap(Sphere)
  (params (OverlappedComponent :type Primitive%20Component%20Object%20Reference) (OtherActor :type Actor%20Object%20Reference) (OtherComp :type Primitive%20Component%20Object%20Reference) (OtherBodyIndex :type Integer))
  (CallFunction|UpdateOverlap OtherActor false))

(event EventBeginPlay
  (|CallParentFunction) ; This node is disabled and will not be called.\nDrag off pins to build functionality.
)

(event Collision|EventActorBeginOverlap
  (params (OtherActor :type Actor%20Object%20Reference))
  (|CallParentFunction OtherActor) ; This node is disabled and will not be called.\nDrag off pins to build functionality.
)

(event EventTick
  (params (DeltaSeconds :type Float%20%28single-precision%29))
  (|CallParentFunction DeltaSeconds) ; This node is disabled and will not be called.\nDrag off pins to build functionality.
)

(event EventInteractwithObject
  (params (Unit :type BP%20Unit%20Base%20Object%20Reference))
  (bind _returnvalue (Game|GetPlayerController 0))
  (CallFunction|UpdateOverlap Unit false)
  (bind _foundwidgets (Widget|GetAllWidgetsOfClass "/Game/Gameplay/UI/WBP_InterestelarMap.WBP_InterestelarMap_C" false))
  (if (<= (Utilities|Array|Length _foundwidgets) 0)
    (bind _returnvalue_2 (UserInterface|CreateWidget "/Game/Gameplay/UI/WBP_InterestelarMap.WBP_InterestelarMap_C"))
    (UserInterface|Viewport|AddtoViewport _returnvalue_2 0)
    (Variables|/Script/Engine.PlayerController|SetbShowMouseCursor _returnvalue true)
    (Input|SetInputModeGameandUI _returnvalue _returnvalue_2 "DoNotLock" true)
    (else
      (for _array_element _foundwidgets
        (Widget|RemovefromParent _array_element))
      (Utilities|Platform|CollectGarbage)
      (Variables|/Script/Engine.PlayerController|SetbShowMouseCursor (Game|GetPlayerController 0) false)
      (Input|SetInputModeGameOnly _returnvalue))))

(fn ConstructionScript
  (|CallParentFunction))