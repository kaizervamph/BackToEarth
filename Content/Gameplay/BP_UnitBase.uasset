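; BP_UnitBase is a unit base Blueprint that holds class, health and a reference to an interaction target.
; On BeginPlay, SetUnitInfo copies the class from the UnitInfo struct and sets both current and max HP from its HP value.
; AnyDamage subtracts from HP while it is above zero, with no clamping or death handling.
; Pressing F applies fixed damage to itself, and SetInteractObject stores the passed actor as InteractActor.
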(event EventBeginPlay
  (CallFunction|SetUnitInfo (Variables|Default|GetUnitInfo)))

(event Collision|EventActorBeginOverlap
  (params (OtherActor :type Actor%20Object%20Reference)))

(event EventTick
  (params (DeltaSeconds :type Float%20%28single-precision%29)))

(event Game|Damage|EventAnyDamage
  (params (Damage :type Float%20%28single-precision%29) (DamageType :type Damage%20Type%20Object%20Reference) (InstigatedBy :type Controller%20Object%20Reference) (DamageCauser :type Actor%20Object%20Reference))
  (if (> (Variables|Default|GetHP) 0.0)
    (Variables|Default|SetHP (- (Variables|Default|GetHP) Damage))))

(event EventSetInteractObject
  (params (Actor :type Actor%20Object%20Reference))
  (Variables|Default|SetInteractActor Actor))

(event Input|KeyboardEvents|F
  (params (Key :type Key%20Structure :default "None"))
  (:Pressed
    (Game|Damage|ApplyDamage self 15.0 0 0)))

(fn ConstructionScript)

(fn SetUnitInfo
  (params (UnitInfo :type Unit%20Struct%20Structure))
  (bind (_class _hp) (Utilities|Struct|BreakUnitStruct UnitInfo))
  (Variables|Default|SetClass _class)
  (Variables|Default|SetHP _hp)
  (Variables|Default|SetHPMAX _hp)
  (return true))