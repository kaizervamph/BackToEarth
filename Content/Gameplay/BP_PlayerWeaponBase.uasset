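; Base player weapon actor that lies as a physics-simulated pickup and fires projectiles.
; An Interaction overlap registers it with the ALS character, and interacting calls PickWeapon on the unit.
; Firing aims from the muzzle, optionally toward a camera-based trace point, then FireWeaponServer plays muzzle effects and spawns projectiles with random pitch/yaw spread.
; A DoOnce gate, reset after ShootDelay, limits the fire rate.
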(event OnComponentBeginOverlap(Interaction)
  (params (OverlappedComponent :type Primitive%20Component%20Object%20Reference) (OtherActor :type Actor%20Object%20Reference) (OtherComp :type Primitive%20Component%20Object%20Reference) (OtherBodyIndex :type Integer) (bFromSweep :type Boolean) (SweepResult :type Hit%20Result%20Structure%20%28by%20ref%29))
  (bind _asals_character_polygon (Utilities|Casting|CastToALS_Character_Polygon OtherActor))
  (Class|IInteract|SetInteractObject(Message) _asals_character_polygon self))

(event OnComponentEndOverlap(Interaction)
  (params (OverlappedComponent :type Primitive%20Component%20Object%20Reference) (OtherActor :type Actor%20Object%20Reference) (OtherComp :type Primitive%20Component%20Object%20Reference) (OtherBodyIndex :type Integer))
  (bind _asals_character_polygon (Utilities|Casting|CastToALS_Character_Polygon OtherActor))
  (Class|IInteract|SetInteractObject(Message) _asals_character_polygon))

(event Custom|FirePlayerWeapon
  (params (UseCameraVector? :type Boolean))
  (Utilities|FlowControl|DoOnce false
    (:Completed
      (CallFunction|FireWeaponServer (CallFunction|GetProjectileSpawnTransform UseCameraVector?)))))

(event Custom|ResetFireWeapon
  (Utilities|FlowControl|DoOnce false) ; enters at Reset
)

(event Custom|SpawnMuzzle
  (Effects|SpawnEmitterAttached (Variables|Default|GetMuzzleVFX) (Variables|Default|GetMuzzle) "None")
  (Audio|PlaySoundatLocation (Variables|Default|GetFireSFX) (Transformation|GetActorLocation) "0, 0, 0" 1.0 1.0 0.0 "/Game/SciFiWeapDark/Sound/Attenuation/WeaponShot_att.WeaponShot_att" 0 0))

(event Custom|FireWeaponServer
  (params (SpawnTransform :type Transform))
  (CallFunction|SpawnMuzzle)
  (for _index (range 1 (Variables|Default|GetProjectilesPerShoot))
    (Game|SpawnActorfromClass (Variables|Default|GetProjectileClass) (CallFunction|RandomizeTransform SpawnTransform false (Variables|Default|GetRangeRandomSpawn)) "AlwaysSpawn" 0 0))
  (Utilities|FlowControl|Delay (Variables|Default|GetShootDelay))
  (CallFunction|ResetFireWeapon))

(event Custom|ChangePhysics
  (params (bSimulate :type Boolean))
  (Physics|SetSimulatePhysics (Variables|Default|GetSkeletalMesh) bSimulate))

(event EventBeginPlay
  (CallFunction|ChangePhysics true))

(event EventInteractwithObject
  (params (Unit :type ALS%20Character%20Polygon%20Object%20Reference))
  (Default|PickWeapon Unit self))

(fn ConstructionScript)

(fn GetProjectileSpawnTransform
  (params (CamVector? :type Boolean))
  (bind _returnvalue (Game|GetPlayerCameraManager 0))
  (bind _muzzle (Variables|Default|GetMuzzle))
  (bind _returnvalue_2 (Camera|GetCameraLocation _returnvalue))
  (bind _returnvalue_3 (Camera|GetCameraRotation _returnvalue))
  (bind _returnvalue_4 (Transformation|GetWorldLocation _muzzle))
  (bind _returnvalue_5 (Math|Vector|GetForwardVector _returnvalue_3))
  (bind _returnvalue_6 (* _returnvalue_5 5e+03))
  (if CamVector?
    (bind _outhit (Collision|LineTraceByChannel _returnvalue_4 (+ _returnvalue_2 (- _returnvalue_6 "450.000000,0.000000,-100.000000")) "TraceTypeQuery5" true 0 "None"))
    (if (.bBlockingHit (Collision|BreakHitResult _outhit))
      (return (Math|Transform|MakeTransform _returnvalue_4 (Math|Rotator|FindLookatRotation _returnvalue_4 (.ImpactPoint (Collision|BreakHitResult _outhit)))))
      (else
        (return (Math|Transform|MakeTransform _returnvalue_4 (Math|Rotator|FindLookatRotation _returnvalue_4 (+ _returnvalue_2 _returnvalue_6))))))
    (else
      (return (Math|Transform|MakeTransform _returnvalue_4 (Transformation|GetWorldRotation _muzzle))))))

(fn RandomizeTransform
  (params (In :type Transform) (Rotation? :type Boolean) (RangeRandomSpawn :type Float%20%28single-precision%29))
  (bind (_location _rotation _scale) (Math|Transform|BreakTransform In))
  (bind _returnvalue (* RangeRandomSpawn -1.0))
  (bind (_roll _pitch _yaw) (Math|Rotator|BreakRotator _rotation))
  (return (Math|Transform|MakeTransform _location (Math|Rotator|MakeRotator _roll (+ _pitch (Math|Random|RandomFloatinRange _returnvalue RangeRandomSpawn)) (+ _yaw (Math|Random|RandomFloatinRange _returnvalue RangeRandomSpawn))) _scale)))