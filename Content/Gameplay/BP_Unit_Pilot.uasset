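; BP_Unit_Pilot is the player's pilot unit, handling gameplay UI, a tablet menu and interaction input.
; It creates the gameplay HUD on begin play.
; Tab flip-flops the tablet: opening creates a new widget, pauses, shows the cursor and sets game-and-UI input, while closing removes all tablet widgets and restores gameplay.
; E sends an interact message to InteractActor when valid, passing itself; this file never sets that reference.
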(event Custom|ToggleTabletUI
  (params (Visibility :type Boolean))
  (bind _returnvalue (Game|GetPlayerController 0))
  (if Visibility
    (bind _returnvalue_2 (UserInterface|CreateWidget "/Game/Gameplay/UI/WBP_TabletUI.WBP_TabletUI_C"))
    (UserInterface|Viewport|AddtoViewport _returnvalue_2 0)
    (Variables|/Script/Engine.PlayerController|SetbShowMouseCursor _returnvalue true)
    (Game|SetGamePaused true)
    (Input|SetInputModeGameandUI _returnvalue _returnvalue_2 "DoNotLock" true)
    (else
      (bind _foundwidgets (Widget|GetAllWidgetsOfClass "/Game/Gameplay/UI/WBP_TabletUI.WBP_TabletUI_C" false))
      (for _array_element _foundwidgets
        (Widget|RemovefromParent _array_element))
      (Variables|/Script/Engine.PlayerController|SetbShowMouseCursor _returnvalue false)
      (Game|SetGamePaused false)
      (Input|SetInputModeGameOnly _returnvalue))))

(event EventBeginPlay
  (|CallParentFunction)
  (bind _returnvalue (UserInterface|CreateWidget "/Game/Gameplay/UI/WBP_GameplayUI.WBP_GameplayUI_C"))
  (UserInterface|Viewport|AddtoViewport _returnvalue 0))

(event Collision|EventActorBeginOverlap
  (params (OtherActor :type Actor%20Object%20Reference)))

(event EventTick
  (params (DeltaSeconds :type Float%20%28single-precision%29))
  (|CallParentFunction DeltaSeconds) ; This node is disabled and will not be called.\nDrag off pins to build functionality.
)

(event Input|KeyboardEvents|E
  (params (Key :type Key%20Structure :default "None"))
  (:Pressed
    (bind _interactactor (Variables|Default|GetInteractActor)
      (:then
        (Class|IInteract|InteractwithObject(Message) _interactactor self))
      (:else))))

(event Input|KeyboardEvents|Tab
  (params (Key :type Key%20Structure :default "None"))
  (:Pressed
    (bind _isa (Utilities|FlowControl|FlipFlop)
      (:A
        _)
      (:B
        _))
    (CallFunction|ToggleTabletUI _isa)))

(fn ConstructionScript
  (|CallParentFunction))