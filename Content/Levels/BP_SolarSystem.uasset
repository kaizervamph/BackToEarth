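; Solar system manager that procedurally generates a few space locations and handles travel between them.
; BeginPlay fills SpaceLocations with random galaxy positions and planet data, built via a macro.
; LoadSpaceLocation fades out, consumes the location by matching its galaxy position, swaps the star sphere material, respawns BP_Planet actors, shows directional lights and fades in.
; Each arrival then spawns a random situation actor from the DT_Situations data table.
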(event Custom|LoadSpaceLocation
  (params (SpaceLocation :type Space%20Location%20Struct%20Structure))
  (bind (_backgroundmaterial _decal1 _decal2 _planets) (Utilities|Struct|BreakSpaceLocationStruct SpaceLocation))
  (bind _returnvalue (Game|GetPlayerController 0))
  (CameraFades|StartCameraFade :self (Variables|/Script/Engine.PlayerController|GetPlayerCameraManager (Game|GetPlayerController 0)) :ToAlpha 1.0 :Duration 1.0 :bHoldWhenFinished true)
  (Utilities|FlowControl|Delay 2.0)
  (bind _success (CallFunction|RemoveSpaceLocation SpaceLocation))
  (if _success
    (Utilities|FlowControl|Sequence
      (:then_0
        (bind _asbp_star_sphere_dynamic (Utilities|Casting|CastToBP_StarSphereDynamic (Variables|/Script/Engine.ChildActorComponent|GetChildActor (Variables|Default|GetBackgroundSpace))))
        (Rendering|Material|SetMaterial (Variables|/Game/StarSphere/Blueprints/BP_StarSphereDynamic.BP_StarSphereDynamic_C|GetStarSphere _asbp_star_sphere_dynamic) 0 _backgroundmaterial))
      (:then_1
        (CallFunction|SpawnPlanets _planets))
      (:then_2
        (bind _outactors (Actor|GetAllActorsOfClass "/Script/Engine.DirectionalLight"))
        (for _array_element _outactors
          (Rendering|SetVisibility (Variables|/Script/Engine.Light|GetLightComponent _array_element) true false))
        (CameraFades|StartCameraFade :self (Variables|/Script/Engine.PlayerController|GetPlayerCameraManager _returnvalue) :FromAlpha 1.0 :Duration 1.0)
        (Variables|/Script/Engine.PlayerController|SetbShowMouseCursor _returnvalue false)
        (CallFunction|RandomSituation)))))

(event Custom|SpawnPlanets
  (params (Planets :type Array%20of%20Planet%20Struct%20Structures))
  (bind _outactors (Actor|GetAllActorsOfClass "/Game/StarSphere/Blueprints/BP_Planet.BP_Planet_C"))
  (for _array_element _outactors
    (Actor|DestroyActor _array_element))
  (for _array_element_2 Planets
    (bind _returnvalue (Game|SpawnActorfromClass "/Game/StarSphere/Blueprints/BP_Planet.BP_Planet_C" (Math|Transform|MakeTransform (* (.Location (Utilities|Struct|BreakPlanetStruct _array_element_2)) 8.0) (Math|Random|RandomRotator false)) "AdjustIfPossibleButAlwaysSpawn" 0 0))
    (Default|SetPlanetInfo _returnvalue (.SurfaceMaterial (Utilities|Struct|BreakPlanetStruct _array_element_2)) (.AtmosphereMaterial (Utilities|Struct|BreakPlanetStruct _array_element_2)))
    (Default|SetDiameter _returnvalue (.Diameter (Utilities|Struct|BreakPlanetStruct _array_element_2)) (.AtmosphereThickness (Utilities|Struct|BreakPlanetStruct _array_element_2)))))

(event Custom|RandomSituation
  (bind _outrownames (DataTable|GetDataTableRowNames "/Game/Data/DT_Situations.DT_Situations"))
  (bind _returnvalue (Utilities|GetDataTableRow "/Game/Data/DT_Situations.DT_Situations" (.OutItem (Utilities|Array|Random _outrownames)))
    (:then
      (bind _returnvalue_2 (Game|SpawnActorfromClass (Utilities|Struct|BreakSituationStruct _returnvalue) (Math|Transform|MakeTransform "0, 0, 0") "AlwaysSpawn" 0 0))
      (Default|SetSituationInfo _returnvalue_2 _returnvalue))))

(event EventBeginPlay
  (bind _spacelocations (CallFunction|GenerateSpaceLocations (Math|Random|RandomIntegerinRange 3 5)))
  (Variables|Default|SetSpaceLocations _spacelocations))

(fn ConstructionScript)

(fn GenerateSpaceLocations
  (params (Amount :type Integer))
  (for _index (range 0 (- Amount 1))
    (bind _planets (Utilities|MGeneratePlanets (Math|Random|RandomIntegerinRange 0 2))
      (:Complete
        (Utilities|Array|Add (LocalVariables|GetTemp) (Utilities|Struct|MakeSpaceLocationStruct "/Game/StarSphere/Materials/MI_StarSphereDynamic_Empty.MI_StarSphereDynamic_Empty" "/Game/StarSphere/Textures/T_Sun.T_Sun" 0 _planets (CallFunction|GetRandomGalaxyLocation))))))
  (return (LocalVariables|GetTemp)))

(fn GetRandomPlanetLocation
  (return (Math|Vector|MakeVector (Math|Random|RandomFloatinRange 2e+04 1e+05) (Math|Random|RandomFloatinRange 2e+04 1e+05) (Math|Random|RandomFloatinRange 2e+04 1e+05))))

(fn GetRandomSurfaceMaterial
  (return (.OutItem (Utilities|Array|Random (Utilities|Array|MakeArray "/Game/StarSphere/Materials/MI_PlanetMarsSurface.MI_PlanetMarsSurface" "/Game/StarSphere/Materials/MI_PlanetVenusSurface.MI_PlanetVenusSurface")))))

(fn GetRandomAtmosphereMaterial
  (return (.OutItem (Utilities|Array|Random (Utilities|Array|MakeArray "/Game/StarSphere/Materials/MI_PlanetMarsAtmosphere.MI_PlanetMarsAtmosphere" "/Game/StarSphere/Materials/MI_PlanetVenusAtmosphere.MI_PlanetVenusAtmosphere")))))

(fn GetRandomGalaxyLocation
  (return (Math|Vector|MakeVector (Math|Random|RandomFloatinRange 2e+04 1e+05) (Math|Random|RandomFloatinRange 2e+04 1e+05) (Math|Random|RandomFloatinRange 2e+04 1e+05))))

(fn RemoveSpaceLocation
  (params (SpaceLocation :type Space%20Location%20Struct%20Structure))
  (for (_array_element _array_index) (Variables|Default|GetSpaceLocations)
    (if (Math|Vector|Equal(Vector) (Utilities|Struct|BreakSpaceLocationStruct _array_element) (Utilities|Struct|BreakSpaceLocationStruct SpaceLocation) 0.0001)
      (Utilities|Array|RemoveIndex (Variables|Default|GetSpaceLocations) _array_index)
      (return true)))
  (return false))