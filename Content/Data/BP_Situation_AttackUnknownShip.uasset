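; Situation Blueprint for an encounter in which an unknown ship attacks.
; On BeginPlay it binds to the play-situation event.
; When that fires, it spawns a BP_Starship_01 at a random distance along the X axis with a flipped rotation and assigns it to team 1.
; It then puts every BP_StarshipBase actor in the world into combat mode.
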(event Custom|OnPlaySituation
  (params (Info :type Situation%20Struct%20Structure))
  (bind _returnvalue (Game|SpawnActorfromClass "/Game/Starships/BP_Starship_01.BP_Starship_01_C" (Math|Transform|MakeTransform (Math|Vector|MakeVector (Math|Random|RandomFloatinRange 1e+04 1e+05) 0.0 0.0) "0,180.000000, 0") "AlwaysSpawn" 0 0))
  (Variables|/Game/Starships/BP_StarshipBase.BP_StarshipBase_C|SetTeam _returnvalue 1)
  (bind _outactors (Actor|GetAllActorsOfClass "/Game/Starships/BP_StarshipBase.BP_StarshipBase_C"))
  (for _array_element _outactors
    (Default|CombatMode _array_element)))

(event EventBeginPlay
  (EventDispatchers|BindEventtoPlaySituation (delegate Custom|OnPlaySituation)))

(fn ConstructionScript
  (|CallParentFunction))